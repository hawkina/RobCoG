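; Player character for a PR2 robot in VR, with eye-level tracking origin, yaw-relative base movement and controller-yaw rotation.
; Arm input axes accumulate into a right end-effector target vector.
; Motion controller triggers set each gripper's opening through a clamped inverse curve, pinned to fully open at rest and closed at full pull.
; Code driving the arm target from the right controller's location is unconnected, as are the bone-location and debug-print snippets.
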(event EventBeginPlay
  ;[1 1 1] Set Tracking origin. If this is not set to eye level, it will be way off and floating above the PR2
  (Class|HeadMountedDisplayFunctionLibrary|SetTrackingOrigin "Eye"))

(event Collision|EventActorBeginOverlap
  (params (OtherActor :type Actor%20Object%20Reference)))

(event EventTick
  (params (DeltaSeconds :type Float%20%28single-precision%29)))

(event Input|AxisEvents|InputAxisMoveArmForward
  (params (AxisValue :type Float%20%28single-precision%29))
  ;[1 1 1] Key Input Arm Control
  (bind _output_get (Variables|Default|Setrx (+ (Variables|Default|Getrx) AxisValue)))
  (Variables|Default|SetRightEndEffectorVector (Math|Vector|MakeVector _output_get (stale Input|AxisEvents|InputAxisMoveArmRight _output_get) (stale Input|AxisEvents|InputAxisMoveArmUp _output_get))))

(event Input|AxisEvents|InputAxisMoveArmRight
  (params (AxisValue :type Float%20%28single-precision%29))
  ;[1 1 1] Key Input Arm Control
  (bind _output_get (Variables|Default|Setry (+ (Variables|Default|Getry) AxisValue)))
  (Variables|Default|SetRightEndEffectorVector (Math|Vector|MakeVector (stale Input|AxisEvents|InputAxisMoveArmForward _output_get) _output_get (stale Input|AxisEvents|InputAxisMoveArmUp _output_get))))

(event Input|AxisEvents|InputAxisMoveArmUp
  (params (AxisValue :type Float%20%28single-precision%29))
  ;[1 1 1] Key Input Arm Control
  (bind _output_get (Variables|Default|Setrz (+ (Variables|Default|Getrz) AxisValue)))
  (Variables|Default|SetRightEndEffectorVector (Math|Vector|MakeVector (stale Input|AxisEvents|InputAxisMoveArmForward _output_get) (stale Input|AxisEvents|InputAxisMoveArmRight _output_get) _output_get)))

(event Input|AxisEvents|InputAxisMoveForward
  (params (AxisValue :type Float%20%28single-precision%29))
  ;[1 1 1] Base Movement
  (Pawn|Input|AddMovementInput (Math|Vector|GetForwardVector (Math|Rotator|MakeRotator 0.0 0.0 (.Yaw (Math|Rotator|BreakRotator (Pawn|GetControlRotation :!class /Script/Engine.Pawn))))) AxisValue false))

(event Input|AxisEvents|InputAxisMoveRight
  (params (AxisValue :type Float%20%28single-precision%29))
  ;[1 1 1] Base Movement
  (Pawn|Input|AddMovementInput (Math|Vector|GetRightVector (Math|Rotator|MakeRotator 0.0 0.0 (.Yaw (Math|Rotator|BreakRotator (Pawn|GetControlRotation :!class /Script/Engine.Pawn))))) AxisValue false))

(event Input|AxisEvents|InputAxisRotateRight
  (params (AxisValue :type Float%20%28single-precision%29))
  ;[1 1 1] Base Movement
  (Pawn|Input|AddControllerYawInput AxisValue))

(event Input|KeyboardEvents|MotionControllerRightTriggerAxis
  (params (AxisValue :type Float%20%28single-precision%29))
  ;[1 1 1] RightGrasp
  ;;[1 1 1] Enforce values 30  and 0 when trigger is not fiering. (Otherwise the controllers spasm out... )
  (if (== AxisValue 0.0)
    (Variables|Default|SetOpenCloseRightGripper 3e+01)
    (elif (== AxisValue 1.0)
      (Variables|Default|SetOpenCloseRightGripper 0.0)
      (else
        (Variables|Default|SetOpenCloseRightGripper (Math|Float|Clamp(Float) (/ 3e+01 (* AxisValue 3e+01)) 0.0 3e+01))))))

(event Input|KeyboardEvents|MotionControllerLeftTriggerAxis
  (params (AxisValue :type Float%20%28single-precision%29))
  ;[1 1 1] LeftGrasp
  ;;[1 1 1] Enforce values 30 and 0 when trigger is not fiering
  (if (== AxisValue 0.0)
    (Variables|Default|SetOpenCloseLeftGripper 3e+01)
    (elif (== AxisValue 1.0)
      (Variables|Default|SetOpenCloseLeftGripper 0.0)
      (else
        (Variables|Default|SetOpenCloseLeftGripper (Math|Float|Clamp(Float) (/ 3e+01 (* AxisValue 3e+01)) 0.0 3e+01))))))

(event Input|KeyboardEvents|MotionControllerRightThumbstick
  (params (Key :type Key%20Structure))
  ;[1 1 1] Base Movement
  ;;[1 1 1] Move base with camera when trackpad is held down on right controller
)

(fn ConstructionScript
  (Variables|Default|SetOpenCloseRightGripper 3e+01)
  (Variables|Default|SetOpenCloseLeftGripper 3e+01))